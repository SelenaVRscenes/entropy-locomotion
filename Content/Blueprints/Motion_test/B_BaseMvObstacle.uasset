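; Base obstacle actor for motion testing, built around a Cylinder component under the scene root.
; The construction script stores the root's world transform as the initial origin, and a function moves the cylinder relative to its parent without sweeping.
; A color getter returns the first vector parameter of the cylinder's material instance.
; The relative-transform getter is an empty stub, and the event graph has no active logic.
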(fn `_F_GetActorMaterialColor`
  (returns (Output_ParameterValue :type "LinearColor Structure"))
  (bind _asmaterial_instance (cast `MaterialInstance` (`PrimitiveComponent.GetMaterial` (`self.Cylinder`) 0)))
  (bind (_output_parameterinfo _output_parametervalue) (break `VectorParameterValue` (`|GetArrayItem` (`MaterialInstance.VectorParameterValues` _asmaterial_instance))))
  (return _output_parametervalue))

(fn `F_Get_ObstacleRelativeTransformToOrign`)

(fn `moveObstacleRelativeToOrign`
  (params (NewLocation :type "Vector Structure"))
  (`SceneComponent.K2_SetRelativeLocation` (`self.Cylinder`) NewLocation false false))

(fn `UserConstructionScript`
  (set `self.InitialWorldOrigin` (`SceneComponent.K2_GetComponentToWorld` (`self.DefaultSceneRoot`))))