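; Industrial double sliding door for the subway train game that opens on a game-instance flag and records player tracking data.
; Tick polls DoorOpenActivate in Store_Vars1, activates both panels, clears the flag and sets ClearBufferGlobal from a trigger counter.
; Component activation plays a timeline that slides the panels apart.
; Each trigger also writes camera location, rotation and timestamp to CSV files named by player, repetition and level.
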(event `self.ReceiveTick`
  (params (DeltaSeconds :type "Float (single-precision)"))
  (bind _returnvalue (`GameplayStatics.GetPlayerCameraManager` 0))
  (bind _returnvalue_2 (`KismetMathLibrary.Now`))
  (bind _levelnamecur (`self.LevelNameCur`))
  (bind _asstore_vars_1 (cast `/Game/Levels/Store_Vars1` (`GameplayStatics.GetGameInstance`)))
  (if (`/Game/Levels/Store_Vars1.DoorOpenActivate` _asstore_vars_1)
    (bind _output_get (set `self.delayCount` (+ (`self.delayCount`) 1)))
    (if (> _output_get 100.0)
      (set `/Game/Levels/Store_Vars1.ClearBufferGlobal` false _asstore_vars_1)
      (else
        (set `/Game/Levels/Store_Vars1.ClearBufferGlobal` true _asstore_vars_1)))
    (`ActorComponent.Activate` (`self.wall_doorway_door_01`) false)
    (`ActorComponent.Activate` (`self.wall_doorway_door_03`) false)
    (bind _asstore_vars_1_2 (cast `/Game/Levels/Store_Vars1` (`GameplayStatics.GetGameInstance`)))
    (set `/Game/Levels/Store_Vars1.DoorOpenActivate` false _asstore_vars_1_2)
    (bind _asstore_vars_1_3 (cast `/Game/Levels/Store_Vars1` (`GameplayStatics.GetGameInstance`)))
    (cast `/Game/Levels/Store_Vars1` (`GameplayStatics.GetGameInstance`))
    (bind _returnvalue_3 (`GameplayStatics.GetCurrentLevelName` true))
    (set `self.LevelNameCur` _returnvalue_3)
    (bind _asstore_vars_1_4 (cast `/Game/Levels/Store_Vars1` (`GameplayStatics.GetGameInstance`)))
    (bind _returnvalue_4 (`KismetStringLibrary.Conv_IntToString` (`/Game/Levels/Store_Vars1.PlayerID` _asstore_vars_1_3)))
    (bind _returnvalue_5 (`KismetStringLibrary.Concat_StrStr` "rep" (`KismetStringLibrary.Conv_IntToString` (`/Game/Levels/Store_Vars1.Count_repet` _asstore_vars_1_4))))
    ;[0.5847 1 0.269] Save to CSV
    (`FPS_Game_Function_Library.WriteLineToCSV` (`KismetStringLibrary.Conv_VectorToString` (`SceneComponent.K2_GetComponentLocation` (`Actor.RootComponent` _returnvalue))) "C:\\temp\\trackingData\\BufferClear" (`KismetStringLibrary.Concat_StrStr` _returnvalue_4 "_" _returnvalue_5 "_" _levelnamecur "_" "Coord.csv"))
    (`FPS_Game_Function_Library.WriteLineToCSV` (`KismetStringLibrary.Conv_RotatorToString` (`SceneComponent.K2_GetComponentRotation` (`Actor.RootComponent` _returnvalue))) "C:\\temp\\trackingData\\BufferClear" (`KismetStringLibrary.Concat_StrStr` _returnvalue_4 "_" _returnvalue_5 "_" _levelnamecur "_" "Angle.csv"))
    (`FPS_Game_Function_Library.WriteLineToCSV` (`KismetStringLibrary.Concat_StrStr` (`KismetStringLibrary.Conv_IntToString` (`KismetMathLibrary.GetYear` _returnvalue_2)) "." (`KismetStringLibrary.Conv_IntToString` (`KismetMathLibrary.GetMonth` _returnvalue_2)) "." (`KismetStringLibrary.Conv_IntToString` (`KismetMathLibrary.GetDay` _returnvalue_2)) "-" (`KismetStringLibrary.Conv_IntToString` (`KismetMathLibrary.GetHour` _returnvalue_2)) "." (`KismetStringLibrary.Conv_IntToString` (`KismetMathLibrary.GetMinute` _returnvalue_2)) "." (`KismetStringLibrary.Conv_IntToString` (`KismetMathLibrary.GetSecond` _returnvalue_2)) "." (`KismetStringLibrary.Conv_IntToString` (`KismetMathLibrary.GetMillisecond` _returnvalue_2))) "C:\\temp\\trackingData\\BufferClear" (`KismetStringLibrary.Concat_StrStr` _returnvalue_4 "_" _returnvalue_5 "_" _levelnamecur "_" "TS.csv"))))

(event `self.wall_doorway_door_01.OnComponentActivated`
  (params (Component :type "ActorComponent Object Reference") (bReset :type Boolean))
  (bind (_direction _newtrack_4) (`Timeline|Door_open`)
    (:`Update`
      (`SceneComponent.K2_SetRelativeLocation` (`self.wall_doorway_door_01`) (`KismetMathLibrary.MakeVector` (+ _newtrack_4 0.0) 10.0 110.0) false false)
      (`SceneComponent.K2_SetRelativeLocation` (`self.wall_doorway_door_03`) (`KismetMathLibrary.MakeVector` (+ (* _newtrack_4 -1.0) -150.0) 10.0 110.0) false false))))

(fn `UserConstructionScript`)