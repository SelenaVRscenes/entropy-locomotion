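; Test obstacle actor that jumps to random positions along the Y axis relative to its origin.
; BeginPlay starts a looping timer at the MotionFramerateS interval to drive the movement.
; Each move picks a random Y within DistanceToCenterRange, keeps X and Z at zero, and calls MoveObstacleRelativeToOrign.
; An optional debug flag prints the Cylinder's relative location in the actor's material color for one interval.
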(event `self.ReceiveBeginPlay`
  (`parent.ReceiveBeginPlay`)
  (`KismetSystemLibrary.K2_SetTimerDelegate` (`|CreateDelegate` :!event `move actor`) (`self.MotionFramerate_s`) true))

(event `move actor`
  (bind (_distancetocenterrange_lowerbound _distancetocenterrange_upperbound) (break `FloatRange` (`self.DistanceToCenterRange`)))
  ;[1 1 1] Move actor to deisred location
  (`self.moveObstacleRelativeToOrign` (`KismetMathLibrary.MakeVector` 0.0 (`KismetMathLibrary.RandomFloatInRange` (`.Value` (break `FloatRangeBound` _distancetocenterrange_lowerbound)) (`.Value` (break `FloatRangeBound` _distancetocenterrange_upperbound)))))
  (if (`self.Debug Move Function`)
    (`self._F_DebugCoordinateMotion` (`SceneComponent.RelativeLocation` (`self.Cylinder`)) (`self.MotionFramerate_s`))))

(fn `_F_DebugCoordinateMotion`
  (params (Location :type "Vector Structure") (`Display Duration` :type "Float (single-precision)"))
  (bind _output_parametervalue (`self._F_GetActorMaterialColor`))
  (`KismetSystemLibrary.PrintString` (`KismetTextLibrary.Conv_TextToString` (`|FormatText` "{value} " (`KismetStringLibrary.Conv_VectorToString` Location))) true true _output_parametervalue `Display Duration`))

(fn `UserConstructionScript`
  (`parent.UserConstructionScript`))