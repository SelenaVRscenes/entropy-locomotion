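; Double sliding door for the subway train level that opens once its DoorActive flag is set; nothing in this Blueprint sets the flag or closes the door.
; Tick polls DoorActive and calls Activate on both door components, using their OnComponentActivated events as the opening trigger.
; Each event plays its own timeline, which slides that leaf along its relative X axis without sweep.
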(event `self.ReceiveTick`
  (params (DeltaSeconds :type "Float (single-precision)"))
  (if (`self.Door_active`)
    (`ActorComponent.Activate` (`self.wall_doorway_door_01`) false)
    (`ActorComponent.Activate` (`self.wall_doorway_door_02`) false)))

(event `self.wall_doorway_door_01.OnComponentActivated`
  (params (Component :type "ActorComponent Object Reference") (bReset :type Boolean))
  (bind (_direction _newtrack_4) (`Timeline|Door_open`)
    (:`Update`
      (`SceneComponent.K2_SetRelativeLocation` (`self.wall_doorway_door_01`) (`KismetMathLibrary.MakeVector` _newtrack_4) false false))))

(event `self.wall_doorway_door_02.OnComponentActivated`
  (params (Component :type "ActorComponent Object Reference") (bReset :type Boolean))
  (bind (_direction _newtrack_1) (`Timeline|Door_open_right`)
    (:`Update`
      (`SceneComponent.K2_SetRelativeLocation` (`self.wall_doorway_door_02`) (`KismetMathLibrary.MakeVector` _newtrack_1) false false))))

(fn `UserConstructionScript`)