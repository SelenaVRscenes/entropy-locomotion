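; Overhead sign light for the subway train that switches from a neutral to a green state on a fixed timer.
; On BeginPlay it hides the ceiling light mesh and tints its point and spot lights grey.
; After a 20-second delay it shows that mesh, hides the default overhead mesh and turns both lights green.
; It then raises the LightOn and HDRIOn flags on the Store_Vars1 game instance.
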(event `self.ReceiveBeginPlay`
  (bind _ceilinglight_300_01 (`self.ceilinglight_300_01`))
  (`PrimitiveComponent.SetEmissiveLightSource` (`self.ceilinglight_300_01`) false)
  (`LightComponent.SetLightColor` (`self.PointLight`) (struct :`R` 0.734375 :`G` 0.734375 :`B` 0.734375 :`A` 1.0) true)
  (`LightComponent.SetLightColor` (`self.SpotLight`) (struct :`R` 0.734375 :`G` 0.734375 :`B` 0.734375 :`A` 1.0) true)
  (`SceneComponent.SetVisibility` _ceilinglight_300_01 false true)
  (`KismetSystemLibrary.Delay` 20.0)
  (`SceneComponent.SetVisibility` _ceilinglight_300_01 true true)
  (`SceneComponent.SetVisibility` (`self.SM_OverheadLight`) false false)
  (`LightComponent.SetLightColor` (`self.PointLight`) (struct :`G` 1.0 :`B` 0.181164 :`A` 1.0) true)
  (`LightComponent.SetLightColor` (`self.SpotLight`) (struct :`G` 1.0 :`B` 0.181164 :`A` 1.0) true)
  (bind _asstore_vars_1 (cast `/Game/Levels/Store_Vars1` (`GameplayStatics.GetGameInstance`)))
  (set `/Game/Levels/Store_Vars1.LightOn` true _asstore_vars_1)
  (set `/Game/Levels/Store_Vars1.HDRI_on` true _asstore_vars_1))

(fn `UserConstructionScript`)