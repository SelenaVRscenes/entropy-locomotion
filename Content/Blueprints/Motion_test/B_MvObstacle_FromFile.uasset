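; Obstacle actor that replays motion from a CSV file and records its position for tracking data.
; BeginPlay parses the file into a runtime DataTable and starts a looping timer to step through rows cyclically, remapping X.
; Tick writes cylinder location and timestamps to CSVs named by player ID, repetition and level from the Store_Vars1 GameInstance.
; A door-open check on Tick tests a constant zero rotation, so it never fires.
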(event `self.ReceiveTick`
  (params (DeltaSeconds :type "Float (single-precision)"))
  (bind _returnvalue (`KismetMathLibrary.Now`))
  (bind _curlevelname (`self.curLevelName`))
  (bind _x (.x (`KismetMathLibrary.Conv_RotatorToVector` (struct))))
  (bind _returnvalue_2 (`KismetStringLibrary.Conv_VectorToString` (`SceneComponent.RelativeLocation` (`self.Cylinder`))))
  (bind _returnvalue_3 (`KismetStringLibrary.Concat_StrStr` (`KismetStringLibrary.Conv_IntToString` (`KismetMathLibrary.GetYear` _returnvalue)) "." (`KismetStringLibrary.Conv_IntToString` (`KismetMathLibrary.GetMonth` _returnvalue)) "." (`KismetStringLibrary.Conv_IntToString` (`KismetMathLibrary.GetDay` _returnvalue)) "-" (`KismetStringLibrary.Conv_IntToString` (`KismetMathLibrary.GetHour` _returnvalue)) "." (`KismetStringLibrary.Conv_IntToString` (`KismetMathLibrary.GetMinute` _returnvalue)) "." (`KismetStringLibrary.Conv_IntToString` (`KismetMathLibrary.GetSecond` _returnvalue)) "." (`KismetStringLibrary.Conv_IntToString` (`KismetMathLibrary.GetMillisecond` _returnvalue))))
  (`parent.ReceiveTick` DeltaSeconds)
  (bind _asstore_vars_1 (cast `/Game/Levels/Store_Vars1` (`GameplayStatics.GetGameInstance`)))
  (bind _asstore_vars_1_2 (cast `/Game/Levels/Store_Vars1` (`GameplayStatics.GetGameInstance`)))
  (bind _returnvalue_4 (`KismetStringLibrary.Conv_IntToString` (`/Game/Levels/Store_Vars1.PlayerID` _asstore_vars_1)))
  (bind _returnvalue_5 (`KismetStringLibrary.Concat_StrStr` "rep" (`KismetStringLibrary.Conv_IntToString` (`/Game/Levels/Store_Vars1.Count_repet` _asstore_vars_1_2))))
  (bind _returnvalue_6 (`KismetStringLibrary.Concat_StrStr` _returnvalue_4 "_" _returnvalue_5 "_" _curlevelname "_" "ObstCoord.csv"))
  (bind _clearbufferglobal (`/Game/Levels/Store_Vars1.ClearBufferGlobal` _asstore_vars_1_2))
  ;[0.5847 1 0.269] Save to CSV
  (`FPS_Game_Function_Library.WriteLineToCSV` _returnvalue_2 "C:\\temp\\trackingData\\Obstacle" _returnvalue_6 _clearbufferglobal)
  (`FPS_Game_Function_Library.WriteLineToCSV` _returnvalue_2 "C:\\temp\\trackingData\\Obstacle\\noBufferClear" _returnvalue_6)
  (bind _returnvalue_7 (`KismetStringLibrary.Concat_StrStr` _returnvalue_4 "_" _returnvalue_5 "_" _curlevelname "_" "TS.csv"))
  (`FPS_Game_Function_Library.WriteLineToCSV` _returnvalue_3 "C:\\temp\\trackingData\\Obstacle\\noBufferClear" _returnvalue_7)
  (`FPS_Game_Function_Library.WriteLineToCSV` _returnvalue_3 "C:\\temp\\trackingData" _returnvalue_7 _clearbufferglobal)
  (if (< _x 0.9999)
    (if (< (`KismetMathLibrary.Abs` (- 1.0 _x)) 0.3)
      (bind _asstore_vars_1_3 (cast `/Game/Levels/Store_Vars1` (`GameplayStatics.GetGameInstance`)))
      (set `/Game/Levels/Store_Vars1.DoorOpenActivate` true _asstore_vars_1_3))))

(event `self.ReceiveBeginPlay`
  (`parent.ReceiveBeginPlay`)
  (`self.LoadFile`)
  ;[1 1 1] Move actor to location
  (`KismetSystemLibrary.K2_SetTimerDelegate` (`|CreateDelegate` :!event `move actor`) (`self.MotionFramerate_s`) true)
  (cast `/Game/Levels/Store_Vars1` (`GameplayStatics.GetGameInstance`))
  (bind _returnvalue (`GameplayStatics.GetCurrentLevelName` true))
  (set `self.curLevelName` _returnvalue))

(event `move actor`
  (bind _motiondatatable (`self.MotionDatatable`))
  ;[1 1 1] Move actor to desired location
  (`/Engine/EditorBlueprintResources/StandardMacros.IsValid` _motiondatatable
    (:`Is Valid`
      ;;[1 1 1] Scale the index to the datatable raw length
      (bind _outrownames (`DataTableFunctionLibrary.GetDataTableRowNames` _motiondatatable))
      (bind _output_get (set `self.timerInt` (mod (`self.timerInt`) (`KismetArrayLibrary.Array_Length` _outrownames))))
      (bind _returnvalue (`KismetStringLibrary.Conv_StringToName` (`KismetStringLibrary.Conv_IntToString` _output_get)))
      (bind _returnvalue_2 (`|GetDataTableRow` (`self.MotionDatatable`) _returnvalue)
        (:`then`
          (bind (_x _y _z) (break `/Game/Blueprints/Motion_test/CustomAnimationStructure` _returnvalue_2))
          (`self.moveObstacleRelativeToOrign` (`KismetMathLibrary.MakeVector` (* (- _x 0.5) 200.0) _y _z))
          (if (`self.Debug Move Function`)
            (`self._F_DebugCoordinateMotion` (`KismetMathLibrary.Conv_IntToDouble` _output_get) (`SceneComponent.RelativeLocation` (`self.Cylinder`)) (`self.MotionFramerate_s`)))
          (`/Engine/EditorBlueprintResources/StandardMacros.IncrementInt` (`self.timerInt`)))
        (:`RowNotFound`
          (`KismetSystemLibrary.PrintText` (`|FormatText` "warning : ROW '{rowName}' was not found within the datatable" _returnvalue) (`self.Print Warning on Screen`) true (struct :`R` 1.0 :`G` 0.593972 :`A` 1.0)))))))

(event `LoadFile`
  (bind _csv_textfile_path_filepath (break `FilePath` (`self.CSV_TextFile_Path`)))
  (bind _csv_textfile_path_filepath_2 (break `FilePath` (`self.CSV_TextFile_Path`)))
  ;[1 1 1] Load data from CSV file
  (if (`FileHelperBPLibrary.IsValidFilename` _csv_textfile_path_filepath_2)
    (if (`BlueprintPathsLibrary.FileExists` _csv_textfile_path_filepath_2)
      ;;[1 0.4675 0.1003] Directly load your CSV textfile inside a DataTable
      (bind (_output _returnvalue) (`FileHelperBPLibrary.ReadText` _csv_textfile_path_filepath))
      (if _returnvalue
        (bind (_success _returnvalue_2) (`FileHelperBPLibrary.CSVToDataTable` _output "/Game/Blueprints/Motion_test/CustomAnimationStructure.CustomAnimationStructure"))
        (if _success
          (set `self.MotionDatatable` _returnvalue_2))))
    (else
      (`KismetSystemLibrary.PrintText` (`|FormatText` "Warning: CSV filepath of {actorNAme} is invalid, no motion possible" (`KismetSystemLibrary.GetObjectName` self)) (`self.Print Warning on Screen`) true (struct :`R` 1.0 :`G` 0.593972 :`A` 1.0) 5.0))))

(fn `_F_DebugCoordinateMotion`
  (params (`time index` :type "Float (double-precision)") (Location :type "Vector Structure") (`Display Duration` :type "Float (single-precision)"))
  (bind _output_parametervalue (`self._F_GetActorMaterialColor`))
  (`KismetSystemLibrary.PrintString` (`KismetTextLibrary.Conv_TextToString` (`|FormatText` "{time} {value} " `time index` (`KismetStringLibrary.Conv_VectorToString` Location))) true true _output_parametervalue `Display Duration`))

(fn `UserConstructionScript`
  (`parent.UserConstructionScript`))